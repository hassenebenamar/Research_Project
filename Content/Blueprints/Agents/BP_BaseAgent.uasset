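; Base agent Blueprint that snaps to the surface below it at spawn and watches for trees.
; BeginPlay's LineTrace temporarily ignores WorldDynamic, traces toward Z zero, then sets height and aligns rotation to the hit normal.
; Tick traces toward the raw forward vector as a world point, ignoring BP_Deer, and calls OnActorOverlap on BP_Tree hits.
; EnvironmentLineTrace provides an unused one-unit forward probe; Tick also draws a debug sphere.
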(event `self.ReceiveBeginPlay`
  (`self.LineTrace`))

(event `self.ReceiveActorBeginOverlap`
  (params (OtherActor :type "Actor Object Reference")))

(event `self.ReceiveTick`
  (params (DeltaSeconds :type "Float (single-precision)"))
  (bind _returnvalue (`self.GetActorForwardVector`))
  (bind _outactors (`GameplayStatics.GetAllActorsOfClass` "/Game/Blueprints/Agents/BP_Deer.BP_Deer_C"))
  (`KismetSystemLibrary.DrawDebugSphere` (+ _returnvalue (200.0 0.0 0.0)) 100.0 24 (struct :`R` 0.020565 :`B` 1.0 :`A` 1.0) 10.0 2.0)
  (bind _outhit (`KismetSystemLibrary.LineTraceSingle` (`self.K2_GetActorLocation`) _returnvalue "TraceTypeQuery1" true _outactors))
  (bind (_bblockinghit _binitialoverlap _time _distance _location _impactpoint _normal _impactnormal _physmat _hitactor) (`GameplayStatics.BreakHitResult` _outhit))
  (if (== (`GameplayStatics.GetObjectClass` _hitactor) "/Game/Blueprints/EnvironmentActors/Trees/BP_Tree.BP_Tree_C")
    (`self.OnActorOverlap` _hitactor)))

(fn `EnvironmentLineTrace`
  (returns (OutHitResult :type "HitResult Structure") (HitOrNo :type Boolean))
  (bind (_outhit _returnvalue) (`KismetSystemLibrary.LineTraceSingle` :`Start` (`self.K2_GetActorLocation`) :`End` (+ (`self.K2_GetActorLocation`) (`self.GetActorForwardVector`)) :`TraceChannel` "TraceTypeQuery1" :`DrawDebugType` "Persistent"))
  (return _outhit _returnvalue))

(fn `LineTrace`
  (bind (_returnvalue_x _returnvalue_y) (`KismetMathLibrary.BreakVector` (`SceneComponent.K2_GetComponentLocation` (`self.CapsuleComponent`))))
  (`PrimitiveComponent.SetCollisionResponseToChannel` (`self.CapsuleComponent`) "ECC_WorldDynamic" "ECR_Ignore")
  (bind _outhit (`KismetSystemLibrary.LineTraceSingle` (`SceneComponent.K2_GetComponentLocation` (`self.CapsuleComponent`)) (`KismetMathLibrary.MakeVector` _returnvalue_x _returnvalue_y) "TraceTypeQuery1"))
  (bind (_bblockinghit _binitialoverlap _time _distance _location _impactpoint _normal) (`GameplayStatics.BreakHitResult` _outhit))
  (`self.K2_SetActorLocation` (+ _location (`KismetMathLibrary.MakeVector` 0.0 0.0 (`CapsuleComponent.GetScaledCapsuleHalfHeight` (`self.CapsuleComponent`)))) true)
  (`self.K2_SetActorRotation` (`KismetMathLibrary.MakeRotFromZX` _normal (`self.GetActorForwardVector`)))
  (`PrimitiveComponent.SetCollisionResponseToChannel` (`self.CapsuleComponent`) "ECC_WorldDynamic" "ECR_Block"))

(fn `UserConstructionScript`)