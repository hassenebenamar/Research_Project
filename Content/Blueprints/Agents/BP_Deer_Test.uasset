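; BP_Deer_Test is a test deer agent Blueprint that can react to heard sounds through AI perception and a Blackboard.
; HandleSoundSense checks a stimulus's sense class and, for hearing only, writes its location to the TargetLocation Blackboard key.
; BeginPlay and construction only call the parent, Tick and overlap are disabled, and nothing in these graphs calls HandleSoundSense.
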(event `self.ReceiveBeginPlay`
  (`parent.ReceiveBeginPlay`))

(fn `HandleSoundSense`
  (params (Stimulus :type "AIStimulus Structure (by ref)"))
  (bind _returnvalue (`AIPerceptionSystem.GetSenseClassForStimulus` Stimulus))
  (if (== _returnvalue "/Script/AIModule.AISense_Hearing")
    (`BlackboardComponent.SetValueAsVector` (`AIBlueprintHelperLibrary.GetBlackboard` null) "TargetLocation" (`.StimulusLocation` (break `AIStimulus` (`local.Stimulus`))))
    (else
      (return))))

(fn `UserConstructionScript`
  (`parent.UserConstructionScript`))