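; BP_Admin is an admin Blueprint that toggles the game's pause menu when the Pause input action is pressed.
; An IsPaused flag picks the branch: pausing creates and shows a PauseMenu widget, pauses the game, and enables game-and-UI input with a visible cursor.
; Unpausing removes the widget, restores game-only input, hides the cursor and resumes play.
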(event `InputAction|Pause` :paused true
  (params (Key :type "Key Structure"))
  (bind _returnvalue (`GameplayStatics.GetPlayerController` 0))
  (bind _returnvalue_2 (`GameplayStatics.GetPlayerController` 0))
  (:`Pressed`
    (if (`self.IsPaused`)
      (`Widget.RemoveFromParent` (stale _returnvalue_3))
      (`WidgetBlueprintLibrary.SetInputMode_GameOnly` _returnvalue)
      (set `PlayerController.bShowMouseCursor` false _returnvalue)
      (`GameplayStatics.SetGamePaused` false)
      (set `self.IsPaused` false)
      (else
        (bind _returnvalue_3 (`|CreateWidget` "/Game/Blueprints/HUD/PauseMenu.PauseMenu_C"))
        (`UserWidget.AddToViewport` _returnvalue_3 0)
        (`GameplayStatics.SetGamePaused` true)
        (`WidgetBlueprintLibrary.SetInputMode_GameAndUIEx` _returnvalue_2 null)
        (set `PlayerController.bShowMouseCursor` true _returnvalue_2)
        (set `self.IsPaused` true)))))

(fn `UserConstructionScript`)